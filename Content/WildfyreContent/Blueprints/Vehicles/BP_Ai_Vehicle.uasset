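; AI-driven vehicle that follows the nearest road spline in either direction, targeting a lane-offset point ahead.
; Each tick it steers by comparing a five-step velocity-predicted path to that target, and adapts max speed to turn sharpness.
; Two front collision volumes cut throttle, with the nearer also triggering the handbrake, as do stop signs.
; Camera-facing text shows speed and steering angle, turning red when braking.
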(event OnComponentBeginOverlap(Collision_Front_Early)
  (params (OverlappedComponent :type Primitive%20Component%20Object%20Reference) (OtherActor :type Actor%20Object%20Reference) (OtherComp :type Primitive%20Component%20Object%20Reference) (OtherBodyIndex :type Integer) (bFromSweep :type Boolean) (SweepResult :type Hit%20Result%20Structure%20%28by%20ref%29))
  (Variables|Default|SetCollForward true))

(event OnComponentBeginOverlap(Collision_Front_Late)
  (params (OverlappedComponent :type Primitive%20Component%20Object%20Reference) (OtherActor :type Actor%20Object%20Reference) (OtherComp :type Primitive%20Component%20Object%20Reference) (OtherBodyIndex :type Integer) (bFromSweep :type Boolean) (SweepResult :type Hit%20Result%20Structure%20%28by%20ref%29))
  (Utilities|FlowControl|Sequence
    (:then_0
      (Variables|Default|SetCollForward true))
    (:then_1
      (Variables|Default|SetCollFwdImminent true))))

(event OnComponentEndOverlap(Collision_Front_Late)
  (params (OverlappedComponent :type Primitive%20Component%20Object%20Reference) (OtherActor :type Actor%20Object%20Reference) (OtherComp :type Primitive%20Component%20Object%20Reference) (OtherBodyIndex :type Integer))
  (Variables|Default|SetCollFwdImminent (> (Utilities|Array|Length (Collision|GetOverlappingActors (Variables|Default|GetCollision_Front_Late) "/Script/Engine.Actor" :!class /Script/Engine.PrimitiveComponent)) 0)))

(event OnComponentEndOverlap(Collision_Front_Early)
  (params (OverlappedComponent :type Primitive%20Component%20Object%20Reference) (OtherActor :type Actor%20Object%20Reference) (OtherComp :type Primitive%20Component%20Object%20Reference) (OtherBodyIndex :type Integer))
  (Variables|Default|SetCollForward (> (Utilities|Array|Length (Collision|GetOverlappingActors (Variables|Default|GetCollision_Front_Early) "/Script/Engine.Actor" :!class /Script/Engine.PrimitiveComponent)) 0)))

(event EventBeginPlay
  (|CallParentFunction)
  (Variables|Default|GetCurrentPath
    (:then
      _)
    (:else
      (CallFunction|AiAcquireRoadSpline)))
  (Utilities|Time|SetTimerbyFunctionName 0 "FindNextTarget" 0.4 true))

(event EventTick
  (params (DeltaSeconds :type Float%20%28single-precision%29))
  (|CallParentFunction DeltaSeconds)
  (Utilities|FlowControl|Sequence
    (:then_0
      (CallFunction|AiUpdateOverheads))
    (:then_1
      (Utilities|FlowControl|Sequence
        (:then_0
          (CallFunction|FindNextTarget))
        (:then_1
          (CallFunction|AiSetSteering))
        (:then_2
          (CallFunction|AiUpdateThrottle))))))

(fn ConstructionScript
  (|CallParentFunction)
  (CallFunction|AiAcquireRoadSpline))

(fn AiStopSign
  (params (MustStop :type Boolean))
  (Variables|Default|SetAiAtStopSign MustStop))

(fn AiUpdateThrottle
  (bind _vehiclemovementcomponent (Variables|Default|GetVehicleMovementComponent))
  (bind _returnvalue (Class|ChaosVehicleMovementComponent|GetHandbrakeInput _vehiclemovementcomponent))
  (Utilities|FlowControl|Sequence
    (:then_0
      (CallFunction|AiAdaptiveTurnSpeed))
    (:then_1
      (LocalVariables|SettIsBraking (Class|ChaosVehicleMovementComponent|GetHandbrakeInput (Variables|Default|GetVehicleMovementComponent)))
      (Class|ChaosVehicleMovementComponent|SetHandbrakeInput (Variables|Default|GetVehicleMovementComponent) (Utilities|ShouldBrake))
      (if (not (== (LocalVariables|GettIsBraking) _returnvalue))
        (Rendering|Components|TextRender|SetTextRenderColor (Variables|Default|GetSpeedometer) (select _returnvalue (Math|Color|MakeColor 0 0 255 255) (Math|Color|MakeColor 255 255 255 255)))))
    (:then_2
      (Class|ChaosVehicleMovementComponent|SetThrottleInput (Variables|Default|GetVehicleMovementComponent) (Math|Float|SelectFloat 0.0 (Math|Float|SelectFloat (Variables|Default|GetThrottlePct) 0.0 (< (* (Math|Float|Absolute(Float) (Vehicle|GetForwardSpeed (Variables|Default|GetVehicleMovementComponent))) 0.036) (Variables|Default|GetAiMaxSpeed))) (Variables|Default|GetCollForward))))))

(fn AiAcquireRoadSpline
  (bind _outactors (Actor|GetAllActorsOfClass "/Game/RC_Roads/Road_Splines/Blueprints/BP_Parent_Spline_Roadways.BP_Parent_Spline_Roadways_C"))
  (Utilities|IsValid (.ReturnValue (Actor|FindNearestActor (Transformation|GetActorLocation) _outactors))
    (:Is%20Valid
      (bind _asbp_parent_spline_roadways (Utilities|Casting|CastToBP_Parent_Spline_Roadways (.ReturnValue (Actor|FindNearestActor (Transformation|GetActorLocation) _outactors))))
      (Variables|Default|SetCurrentPath _asbp_parent_spline_roadways))
    (:Is%20Not%20Valid
      (Development|PrintString "No Road Spline Detected. There WILL be problems!" true true "(R=1.000000,G=0.000000,B=0.000000,A=1.000000)" 5.0))))

(fn AiSetSteering
  (CallFunction|AiSetTargetVector)
  (CallFunction|AiPredictPath)
  (Class|ChaosVehicleMovementComponent|SetSteeringInput (Variables|Default|GetVehicleMovementComponent) (Variables|Default|GetAiSteeringOffset)))

(fn AiUpdateOverheads
  (Utilities|FlowControl|Sequence
    (:then_0
      (Transformation|SetWorldRotation (Variables|Default|GetScene1) (Math|Rotator|FindLookatRotation (Transformation|GetWorldLocation (Variables|Default|GetScene1)) (Transformation|GetActorLocation (Game|GetPlayerCameraManager 0))) false false))
    (:then_1
      (Rendering|Components|TextRender|SetText (Variables|Default|GetSpeedometer) (Utilities|Text|FormatText "{mph} MPH" (Math|Float|Round (Class|ChaosVehicleMovementComponent|GetForwardSpeedMPH (Variables|Default|GetVehicleMovementComponent))))))
    (:then_2
      (bind _returnvalue (Class|ChaosVehicleMovementComponent|GetSteeringInput (Variables|Default|GetVehicleMovementComponent)))
      (Rendering|Components|TextRender|SetText (Variables|Default|GetSteeringAngle) (Utilities|Text|FormatText "{steer}°{LR}" (Math|Integer|Absolute(Integer) (Math|Float|Round (* _returnvalue (LocalVariables|GettDegreesSteering)))) (Utilities|String|SelectText "L" "R" (< _returnvalue 0.0)))))))

(fn AiSteeringAngle
  (bind (_isleftofvehicle _leftdistance _rightdistance _difffromleft) (Utilities|IsRightorLeftOfVehicle))
  (Variables|Default|SetAiSteeringOffset (Math|Float|Lerp (Variables|Default|GetAiSteeringOffset) (* (Math|Float|SelectFloat 0.65 -0.65 _isleftofvehicle) (Math|Float|SelectFloat 0.0 1.0 (and (< (Math|Float|Absolute(Float) _difffromleft) (LocalVariables|GettSteeringGap)) (.IsBehind (Utilities|IsAheadorBehindVehicle))))) (* (Utilities|Time|GetWorldDeltaSeconds) 4e+01))))

(fn AiSetTargetVector
  (bind _output_get (Variables|Default|SetTargetVector (Utilities|GetTargetSplineDistance)))
  (Utilities|FlowControl|Sequence
    (:then_0
      (if (< (Math|Vector|Distance(Vector) _output_get (Transformation|GetActorLocation)) (Variables|Default|GetCheckGap))
        (Utilities|SetSplineDistance)))
    (:then_1
      (if (Variables|Default|GetShowDebugging)
        (Rendering|Debug|DrawDebugLine (Transformation|GetActorLocation) (Variables|Default|GetTargetVector) "(R=1.000000,G=0.000000,B=0.410392,A=1.000000)" 0.0 5.0)))))

(fn FindNextTarget
  (Variables|Default|GetCurrentPath
    (:then
      (if (< (Math|Vector|Distance(Vector) (Spline|GetLocationatDistanceAlongSpline (Variables|/Game/RC_Roads/Road_Splines/Blueprints/BP_Parent_Spline_Roadways.BP_Parent_Spline_Roadways_C|GetSpline (Variables|Default|GetCurrentPath)) (LocalVariables|GettSplineDistance) "World") (Transformation|GetActorLocation)) (LocalVariables|GettDistanceClosestPoint)) :!label _label
        (LocalVariables|SettDistanceClosestPoint (Math|Vector|Distance(Vector) (Spline|GetLocationatDistanceAlongSpline (Variables|/Game/RC_Roads/Road_Splines/Blueprints/BP_Parent_Spline_Roadways.BP_Parent_Spline_Roadways_C|GetSpline (Variables|Default|GetCurrentPath)) (LocalVariables|GettSplineDistance) "World") (Transformation|GetActorLocation)))
        (LocalVariables|SettClosestSplineDistance (LocalVariables|GettSplineDistance)))
      (bind _output_get (LocalVariables|SettSplineDistance (+ (LocalVariables|GettSplineDistance) 1e+03)))
      (if (> _output_get (Utilities|GetSplineLength))
        (if (Variables|Default|GetDriveForward)
          (Variables|Default|SetTargetSplineDist (Math|Float|SelectFloat 0.0 (+ (LocalVariables|GettClosestSplineDistance) (LocalVariables|GettTargetSearchDistance)) (> (+ (LocalVariables|GettClosestSplineDistance) (LocalVariables|GettTargetSearchDistance)) (Utilities|GetSplineLength))))
          (else
            (Variables|Default|SetTargetSplineDist (Math|Float|SelectFloat (Utilities|GetSplineLength) (- (LocalVariables|GettClosestSplineDistance) (LocalVariables|GettTargetSearchDistance)) (< (- (LocalVariables|GettClosestSplineDistance) (LocalVariables|GettTargetSearchDistance)) 0.0)))))
        (else
          (goto _label))))
    (:else)))

(fn AiAdaptiveTurnSpeed
  (bind _returnvalue (Transformation|GetActorLocation))
  (bind _returnvalue_2 (Transformation|GetActorRotation))
  (bind _targetvector (Variables|Default|GetTargetVector))
  (bind _aisensitivityturncaution (Variables|Default|GetAiSensitivityTurnCaution))
  (bind _returnvalue_3 (Math|Rotator|FindLookatRotation _returnvalue _targetvector))
  (bind _returnvalue_4 (Math|Rotator|Delta(Rotator) _returnvalue_3 _returnvalue_2))
  (bind _returnvalue_5 (Math|Float|Absolute(Float) (.yaw _returnvalue_4)))
  (bind _returnvalue_6 (/ _aisensitivityturncaution _returnvalue_5))
  (Variables|Default|SetAiMaxSpeed (Math|Float|Clamp(Float) (Math|Float|Lerp (Variables|Default|GetAiMaxSpeed) _returnvalue_6 (* (Utilities|Time|GetWorldDeltaSeconds) (Math|Float|SelectFloat (Variables|Default|GetAiSensitivityTurnBraking) 1.0 (> (Variables|Default|GetAiMaxSpeed) _returnvalue_6)))) 4.0 8e+01)))

(fn AiPredictPath
  (bind _returnvalue (Transformation|GetActorLocation))
  (bind _returnvalue_2 (Transformation|GetActorLocation))
  (Utilities|FlowControl|Sequence
    (:then_0
      (LocalVariables|SettPredictedVector _returnvalue)
      (LocalVariables|SettVelocity (Transformation|GetVelocity))
      (LocalVariables|SettTimeStep (/ (/ (Math|Vector|Distance(Vector) _returnvalue (Variables|Default|GetTargetVector)) (Math|Vector|VectorLength (LocalVariables|GettVelocity))) 5.0)))
    (:then_1
      (LocalVariables|SettSteerYawOffset (.yaw (Math|Rotator|Delta(Rotator) (Math|Conversions|RotationFromXVector (Math|Vector|Normalize (LocalVariables|GettVelocity))) (Transformation|GetActorRotation))))
      (for _index (range 1 5)
        (LocalVariables|SettPredictedVector (+ (LocalVariables|GettPredictedVector) (* (LocalVariables|GettVelocity) (LocalVariables|GettTimeStep))))
        (LocalVariables|SettVelocity (Math|Vector|RotateVectorAroundAxis (LocalVariables|GettVelocity) (LocalVariables|GettSteerYawOffset) "0.000000,0.000000,1.000000")))
      (Variables|Default|SetAiSteeringOffset (Math|Float|Clamp(Float) (* (.yaw (Math|Rotator|Delta(Rotator) (Math|Rotator|FindLookatRotation _returnvalue_2 (LocalVariables|GettPredictedVector)) (Math|Rotator|FindLookatRotation _returnvalue_2 (Variables|Default|GetTargetVector)))) -0.1) -1.0)))))

(fn AiCorneringForce
  (params (InTurnRadius :type Float%20%28double-precision%29))
  (bind _mesh (Variables|Character|GetMesh))
  (bind _returnvalue (Physics|GetMass _mesh))
  (return (Math|Float|Sqrt (/ (* (* (LocalVariables|GettCornerStiff) (LocalVariables|GettFrictionForce)) InTurnRadius) _returnvalue)) (/ (* _returnvalue (Math|Float|Square (Vehicle|GetForwardSpeed (Variables|Default|GetVehicleMovementComponent)))) InTurnRadius)))