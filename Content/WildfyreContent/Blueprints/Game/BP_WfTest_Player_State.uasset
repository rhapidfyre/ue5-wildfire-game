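; BP_WfTest_Player_State is a test player state that sets up a basic vehicle and team for the player at BeginPlay.
; It stores the first fire station found, waits briefly, then purchases the "medic" apparatus from the DT_Fleet_Purchase data table.
; It then converts the first two entries in the game mode's transfer list into job contracts and accepts them to form the team.
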(event EventBeginPlay
  (|CallParentFunction)
  (Utilities|FlowControl|Sequence
    (:then_0
      (Development|PrintString "BP_WfTest_Player_State is initializing a basic vehicle and team"))
    (:then_1
      (bind _outactors (Actor|GetAllActorsOfClass "/Script/ProjectWildfire.WfFireStationBase"))
      (Class|WfPlayerStateBase|SetFireStationReference (Utilities|Array|Get(acopy) _outactors))
      (Utilities|FlowControl|Delay 3.0)
      (Utilities|FlowControl|Sequence
        (:then_0
          (bind _returnvalue (Utilities|GetDataTableRow "/Game/WildfyreContent/Data/DT_Fleet_Purchase.DT_Fleet_Purchase" "medic")
            (:then
              (Class|WfPlayerStateBase|PurchaseFireApparatus _returnvalue))))
        (:then_1
          (bind _aswf_game_mode_base (Utilities|Casting|CastToWfGameModeBase (Game|GetGameMode)))
          (bind _returnvalue_2 (Class|WfGameModeBase|ConvertSavetoJobContract (Utilities|Array|Get(acopy) (Class|WfGameModeBase|GetListOfTransfers _aswf_game_mode_base) 1)))
          (Class|WfPlayerStateBase|AcceptJobContract _returnvalue_2)
          (bind _returnvalue_3 (Class|WfGameModeBase|ConvertSavetoJobContract (Utilities|Array|Get(acopy) (Class|WfGameModeBase|GetListOfTransfers _aswf_game_mode_base))))
          (Class|WfPlayerStateBase|AcceptJobContract _returnvalue_3))))))

(fn ConstructionScript)