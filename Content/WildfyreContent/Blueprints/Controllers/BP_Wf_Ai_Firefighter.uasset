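; AI controller for firefighter characters that runs the generic AI behavior tree and blackboard.
; On BeginPlay it retries every 0.2 seconds until the controlled pawn is a WfFfCharacterBase, then caches the character and its ability component.
; It binds to the component's attribute-change event to copy thirst and hunger values into the blackboard as they change.
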(event Custom|Init_AiCharacter
  (bind _aswf_ff_character_base (Utilities|Casting|CastToWfFfCharacterBase (Pawn|GetControlledPawn))
    (:then
      (bind _output_get (Variables|Default|SetCharacterReference _aswf_ff_character_base))
      (Utilities|FlowControl|Sequence
        (:then_0
          (bind _aswf_ability_component (Utilities|Casting|CastToWfAbilityComponent (Ability|GetAbilitySystemComponent _output_get)))
          (Variables|Default|SetAbilityComponent _aswf_ability_component)
          (EventDispatchers|BindEventtoOnAttributeChanged _aswf_ability_component (EventDispatchers|CreateEvent :!event Custom|Callback_AttributeChanged)))
        (:then_1
          (Class|AIController|UseBlackboard "/Game/WildfyreContent/Behaviors/BB_Ai_Generic.BB_Ai_Generic")
          (AI|RunBehaviorTree "/Game/WildfyreContent/Behaviors/BT_Ai_Generic.BT_Ai_Generic"))))
    (:CastFailed
      (Utilities|FlowControl|Delay 0.2)
      (CallFunction|InitAiCharacter))))

(event Custom|Callback_AttributeChanged
  (params (GameAttribute :type Gameplay%20Attribute%20Structure%20%28by%20ref%29) (OldValue :type Float%20%28single-precision%29) (NewValue :type Float%20%28single-precision%29))
  (bind _returnvalue (AI|GetBlackboard 0))
  (bind _abilitycomponent (Variables|Default|GetAbilityComponent))
  (if (== GameAttribute "(AttributeName=\"Thirst\",Attribute=/Script/ProjectWildfire.WfAttributeSet:Thirst,AttributeOwner=\"/Script/CoreUObject.Class'/Script/ProjectWildfire.WfAttributeSet'\")")
    (AI|Components|Blackboard|SetValueasFloat _returnvalue (Utilities|Name|MakeLiteralName "ThirstValue") (.ReturnValue (Class|AbilitySystemComponent|GetGameplayAttributeValue _abilitycomponent "(AttributeName=\"Thirst\",Attribute=/Script/ProjectWildfire.WfAttributeSet:Thirst,AttributeOwner=\"/Script/CoreUObject.Class'/Script/ProjectWildfire.WfAttributeSet'\")")))
    (elif (== GameAttribute "(AttributeName=\"Hunger\",Attribute=/Script/ProjectWildfire.WfAttributeSet:Hunger,AttributeOwner=\"/Script/CoreUObject.Class'/Script/ProjectWildfire.WfAttributeSet'\")")
      (AI|Components|Blackboard|SetValueasFloat _returnvalue (Utilities|Name|MakeLiteralName "HungerValue") (.ReturnValue (Class|AbilitySystemComponent|GetGameplayAttributeValue _abilitycomponent "(AttributeName=\"Hunger\",Attribute=/Script/ProjectWildfire.WfAttributeSet:Hunger,AttributeOwner=\"/Script/CoreUObject.Class'/Script/ProjectWildfire.WfAttributeSet'\")"))))))

(event EventBeginPlay
  (CallFunction|InitAiCharacter))

(fn ConstructionScript)