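; AI driver controller that steers a possessed WfVehicleBase along the first RoadSpline found in the level.
; Each tick it aims at the spline point nearest a tangent-based look-ahead and maps yaw error to steering.
; Throttle is on/off against TargetSpeed, whose index in SpeedLimits also sets the gear.
; A debug timer cycles speed limits, number keys set fixed targets, and Blackboard setup is unconnected.
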(event Custom|Init_VehicleReference
  (bind _aswf_vehicle_base (Utilities|Casting|CastToWfVehicleBase (Pawn|GetControlledPawn))
    (:then
      (Variables|Default|SetVehicleReference _aswf_vehicle_base)
      (Utilities|FlowControl|Sequence))
    (:CastFailed
      (Utilities|FlowControl|Delay 0.2)
      (CallFunction|InitVehicleReference))))

(event Custom|Debug_SpeedChanger
  (bind _output_get (Variables|Default|SetDebugSpeedIndex (Math|Integer|SelectInt 0 (+ (Variables|Default|GetDebugSpeedIndex) 1) (> (+ (Variables|Default|GetDebugSpeedIndex) 1) (Utilities|Array|LastIndex (Variables|Default|GetSpeedLimits))))))
  (bind _output_get_2 (Variables|Default|SetTargetSpeed (Utilities|Array|Get(acopy) (Variables|Default|GetSpeedLimits) _output_get)))
  (Development|PrintString (Utilities|String|Append "Max Speed Set: " (Utilities|String|ToString(Integer) (Math|Float|Round _output_get_2)) "m/s") true true "(R=1.000000,G=0.433389,B=0.000000,A=1.000000)"))

(event EventBeginPlay
  (CallFunction|InitVehicleReference)
  (Utilities|Time|SetTimerbyEvent (delegate Custom|Debug_SpeedChanger) 5.0 true))

(event EventTick
  (params (DeltaSeconds :type Float%20%28single-precision%29))
  (Variables|Default|GetActivePath
    (:then
      (bind _returnvalue (CallFunction|GetVehiclePath))
      (Class|ChaosVehicleMovementComponent|SetSteeringInput (Variables|/Script/ChaosVehicles.WheeledVehiclePawn|GetVehicleMovementComponent (Variables|Default|GetVehicleReference)) _returnvalue)
      (CallFunction|ControlSpeed))
    (:else
      (bind _returnvalue_2 (Actor|GetActorOfClass "/Game/WildfyreContent/Blueprints/RoadSpline.RoadSpline_C"))
      (Variables|Default|SetActivePath _returnvalue_2))))

(event Input|KeyboardEvents|1
  (params (Key :type Key%20Structure :default "None"))
  (:Pressed
    (Variables|Default|SetTargetSpeed 25.0)))

(event Input|KeyboardEvents|2
  (params (Key :type Key%20Structure :default "None"))
  (:Pressed
    (Variables|Default|SetTargetSpeed 8e+01)))

(event Input|KeyboardEvents|3
  (params (Key :type Key%20Structure :default "None"))
  (:Pressed
    (Variables|Default|SetTargetSpeed 165.0)))

(fn ConstructionScript)

(fn GetVehiclePath
  (bind _vehiclereference (Variables|Default|GetVehicleReference))
  (bind _returnvalue (Transformation|GetActorLocation _vehiclereference))
  (bind _activepath (Variables|Default|GetActivePath)
    (:then
      (return (Math|Float|MapRangeClamped (.yaw (Math|Rotator|Delta(Rotator) (Math|Rotator|FindLookatRotation _returnvalue (Spline|FindLocationClosesttoWorldLocation (Variables|/Game/WildfyreContent/Blueprints/RoadSpline.RoadSpline_C|GetSpline (Variables|Default|GetActivePath)) (+ (* (Math|Vector|Normalize (Class|SplineComponent|FindTangentClosesttoWorldLocation (Variables|/Game/WildfyreContent/Blueprints/RoadSpline.RoadSpline_C|GetSpline _activepath) (Transformation|GetActorLocation (Variables|Default|GetVehicleReference)) "World")) 2e+02) _returnvalue) "World")) (Transformation|GetActorRotation _vehiclereference))) -9e+01 9e+01 -1.0 1.0)))
    (:else
      (return 0.0))))

(fn ControlSpeed
  (bind _vehiclereference (Variables|Default|GetVehicleReference))
  (bind _vehiclereference_2 (Variables|Default|GetVehicleReference))
  (bind _vehiclemovementcomponent (Variables|/Script/ChaosVehicles.WheeledVehiclePawn|GetVehicleMovementComponent _vehiclereference))
  (bind _vehiclemovementcomponent_2 (Variables|/Script/ChaosVehicles.WheeledVehiclePawn|GetVehicleMovementComponent _vehiclereference_2))
  (for (_array_element _array_index) (Variables|Default|GetSpeedLimits)
    (if (== _array_element (Variables|Default|GetTargetSpeed))
      (Class|ChaosVehicleMovementComponent|SetTargetGear _vehiclemovementcomponent_2 _array_index true)
      (if (> (* (Vehicle|GetForwardSpeed _vehiclemovementcomponent_2) 0.036) (Variables|Default|GetTargetSpeed))
        (Class|ChaosVehicleMovementComponent|SetThrottleInput _vehiclemovementcomponent 0.0)
        (else
          (Class|ChaosVehicleMovementComponent|SetThrottleInput _vehiclemovementcomponent 1.0))))))