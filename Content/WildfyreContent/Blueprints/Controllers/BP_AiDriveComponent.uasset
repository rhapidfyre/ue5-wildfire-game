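; AI controller component that lets AI characters enter and exit vehicles by seat.
; It caches controller and character on begin play, retrying until valid.
; EnterVehicle writes blackboard movement targets when out of reach; otherwise, or when forced, it possesses the vehicle and attaches the collisionless character to the driver socket.
; ExitVehicle detaches, teleports and repossesses the character; StartDriving and reference setup/cleanup are empty stubs.
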(event Custom|StartDriving)

(event Custom|Init_ControllerReference
  ;[0.1 0.1 0.1 0.4] Init Controller Reference
  (bind _asbp_ai_controller (Utilities|Casting|CastToBP_Ai_Controller (Components|GetOwner))
    (:then
      (Variables|Default|SetAiController _asbp_ai_controller))
    (:CastFailed
      (Utilities|FlowControl|Delay 0.2)
      (CallFunction|InitControllerReference))))

(event Custom|InitOriginalCharacter
  (bind _aicontroller (Variables|Default|GetAiController)
    (:then
      (bind _aicharacter (Variables|/Game/WildfyreContent/Blueprints/Controllers/BP_Ai_Controller.BP_Ai_Controller_C|GetAiCharacter _aicontroller)
        (:then
          (Variables|Default|SetCharacterReference _aicharacter))
        (:else
          (Utilities|FlowControl|Delay 0.2 :!label _label)
          (CallFunction|InitOriginalCharacter))))
    (:else
      (goto _label))))

(event EventBeginPlay
  (|CallParentFunction)
  (CallFunction|InitControllerReference)
  (CallFunction|InitOriginalCharacter))

(fn SetVehicleinUse
  (params (VehicleReference :type Wf%20Vehicle%20Base%20Object%20Reference))
  (Utilities|FlowControl|Sequence
    (:then_0
      (CallFunction|CleanReferences))
    (:then_1
      (Variables|Default|SetVehicleReference VehicleReference)
      (CallFunction|SetupReferences))
    (:then_2
      (Variables|Default|SetIsUsingVehicle (Utilities|IsValid VehicleReference)))
    (:then_3
      (Development|PrintString (Utilities|String|Append (Utilities|GetDisplayName (Variables|Default|GetAiController)) ": I am " (Utilities|String|SelectString (Utilities|String|Append "now driving " (Utilities|GetDisplayName (Variables|Default|GetVehicleReference))) "no longer driving." (Variables|Default|GetIsUsingVehicle))) true true "(R=0.000000,G=0.660000,B=1.000000,A=1.000000)" 3.0))))

(fn CleanReferences
  (Variables|Default|GetVehicleReference
    (:then)
    (:else)))

(fn SetupReferences
  (Variables|Default|GetVehicleReference
    (:then)
    (:else)))

(fn EnterVehicle
  (params (InVehicle :type Wf%20Vehicle%20Base%20Object%20Reference) (InSeatNumber :type Integer) (ForcedEnter :type Boolean))
  (bind _aicontroller (Variables|Default|GetAiController))
  (bind _aicontroller_2 (Variables|Default|GetAiController))
  (bind _returnvalue (AI|GetBlackboard _aicontroller))
  (bind (_isinreach _outvector) (Utilities|GetSeatEnterVector InVehicle InSeatNumber))
  (bind _aicharacter (Variables|/Game/WildfyreContent/Blueprints/Controllers/BP_Ai_Controller.BP_Ai_Controller_C|GetAiCharacter _aicontroller_2))
  (Utilities|IsValid InVehicle
    (:Is%20Valid
      (Variables|AiBehavior|SetIsEnteringVehicle true)
      (Variables|Default|SetUsingSeat InSeatNumber)
      (Utilities|FlowControl|Sequence
        (:then_0
          ;[0.1 0.1 0.1 0.4 14] Too far away & "Forced Enter" is also false
          (if (and (not ForcedEnter) (not _isinreach))
            ;[0.1 0.1 0.1 0.4 14] Move to the vehicle's entry vector
            (AI|Components|Blackboard|SetValueasVector _returnvalue (Utilities|Name|MakeLiteralName "TargetDestination") _outvector)
            (AI|Components|Blackboard|SetValueasObject _returnvalue (Utilities|Name|MakeLiteralName "InteractionTarget") InVehicle)
            (Class|BlackboardComponent|SetValueasInt _returnvalue (Utilities|Name|MakeLiteralName "VehicleSeat") InSeatNumber)
            (else
              (Variables|AiBehavior|SetIsEnteringVehicle false) ; Vehicle in Reach
              (CallFunction|SetVehicleinUse InVehicle)
              (Class|WfVehicleBase|SetSeatOccupant (Variables|Default|GetVehicleReference) (Variables|Default|GetUsingSeat) (Variables|Default|GetCharacterReference))
              (Pawn|Possess (Variables|Default|GetAiController) (Variables|Default|GetVehicleReference))
              (Collision|SetActorEnableCollision _aicharacter false)
              (Transformation|AttachComponentToComponent _aicharacter (Variables|/Script/ChaosVehicles.WheeledVehiclePawn|GetMesh (Variables|Default|GetVehicleReference)) "Seat_Driver" "SnapToTarget" "SnapToTarget" "KeepWorld" true))))
        (:then_1
          (Default|CallOnVehicleEntered InVehicle (Variables|Default|GetUsingSeat) (not (Variables|AiBehavior|GetIsEnteringVehicle))))))))

(fn ExitVehicle
  (bind _vehiclereference (Variables|Default|GetVehicleReference))
  (bind _aicontroller (Variables|Default|GetAiController))
  (bind _aicontroller_2 (Variables|Default|GetAiController))
  (bind _aicharacter (Variables|/Game/WildfyreContent/Blueprints/Controllers/BP_Ai_Controller.BP_Ai_Controller_C|GetAiCharacter _aicontroller))
  (bind _aicharacter_2 (Variables|/Game/WildfyreContent/Blueprints/Controllers/BP_Ai_Controller.BP_Ai_Controller_C|GetAiCharacter _aicontroller_2))
  (Variables|AiBehavior|SetIsEnteringVehicle false) ; Stop trying to enter vehicles
  (Utilities|IsValid _vehiclereference
    (:Is%20Valid
      (LocalVariables|SettOldVehicle _vehiclereference)
      (Utilities|FlowControl|Sequence
        (:then_0
          ;[0.1 0.1 0.1 0.4 14] Enable Collisions & Move Character out of the vehicle
          (Transformation|DetachFromActor _aicharacter "KeepWorld" "KeepWorld" "KeepWorld")
          (Collision|SetActorEnableCollision _aicharacter true))
        (:then_1
          (Transformation|SetActorLocation (Variables|/Game/WildfyreContent/Blueprints/Controllers/BP_Ai_Controller.BP_Ai_Controller_C|GetAiCharacter (Variables|Default|GetAiController)) (Utilities|GetSeatExitVector (LocalVariables|GettOldVehicle) (.SeatNumber (CallFunction|GetSeatNumber))) false true))
        (:then_2
          (Pawn|Possess _aicontroller_2 _aicharacter_2)
          (Class|WfVehicleBase|SetSeatOccupant (LocalVariables|GettOldVehicle) (Variables|Default|GetUsingSeat) _aicharacter_2)
          (Variables|Default|SetUsingSeat -1)
          (CallFunction|SetVehicleinUse))))
    (:Is%20Not%20Valid
      (Variables|Default|SetUsingSeat -1))))

(fn GetSeatNumber
  (return (Utilities|IsValid (Variables|Default|GetVehicleReference)) (Variables|Default|GetUsingSeat)))