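; AI controller for Wildfyre characters that starts the generic AI behavior tree on the controlled pawn.
; On BeginPlay it casts the pawn to WfCharacterBase, retrying after a short delay until that succeeds, then caches it and runs BT_Ai_Generic.
; It also stores an assigned vehicle through an event.
; ControlSpeed looks unfinished, with no array input and zero throttle on both branches, and GetStationLocation has only unused nodes.
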(event Custom|InitAiCharacter
  (bind _aswf_character_base (Utilities|Casting|CastToWfCharacterBase (Pawn|GetControlledPawn))
    (:then
      (Variables|Default|SetAiCharacter _aswf_character_base)
      (AI|RunBehaviorTree "/Game/WildfyreContent/Behaviors/BT_Ai_Generic.BT_Ai_Generic"))
    (:CastFailed
      (Utilities|FlowControl|Delay 0.2)
      (CallFunction|InitAiCharacter))))

(event Custom|SetAssignedVehicle
  (params (NewVehicle :type Wf%20Fire%20Apparatus%20Base%20Object%20Reference))
  (Variables|Default|SetVehicleAssigned NewVehicle))

(event EventBeginPlay
  (|CallParentFunction)
  (CallFunction|InitAiCharacter))

(fn ConstructionScript)

(fn ControlSpeed
  (bind _vehiclereference (Variables|Default|GetVehicleReference))
  (bind _vehiclereference_2 (Variables|Default|GetVehicleReference))
  (bind _vehiclemovementcomponent (Variables|/Script/ChaosVehicles.WheeledVehiclePawn|GetVehicleMovementComponent _vehiclereference))
  (bind _vehiclemovementcomponent_2 (Variables|/Script/ChaosVehicles.WheeledVehiclePawn|GetVehicleMovementComponent _vehiclereference_2))
  (for (_array_element _array_index) 0
    (if (== _array_element 0.0)
      (Class|ChaosVehicleMovementComponent|SetTargetGear _vehiclemovementcomponent_2 _array_index true)
      (if (> (* (Vehicle|GetForwardSpeed _vehiclemovementcomponent_2) 0.036) 0.0)
        (Class|ChaosVehicleMovementComponent|SetThrottleInput _vehiclemovementcomponent 0.0)
        (else
          (Class|ChaosVehicleMovementComponent|SetThrottleInput _vehiclemovementcomponent 0.0))))))