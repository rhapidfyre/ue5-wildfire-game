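; Player HUD Blueprint that builds and displays the game's on-screen widgets.
; BeginPlay creates a message box, then waits for the Wildfyre player controller before adding the bottom toolbar, selected-actor panel, clock and side-bar menus.
; Controller, game state and player state checks retry on short delays until their casts succeed.
; SendMessage shows titled, leveled alerts with a fallback icon, and a delayed load notice uses it.
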(event Custom|Init_PlayerController
  (Utilities|Casting|CastToWfPlayerControllerBase (Game|GetPlayerController 0)
    (:then
      (CallFunction|InitToolbar)
      (CallFunction|InitSelectedActor)
      (CallFunction|InitWeatherData)
      (CallFunction|InitPrimaryMenus))
    (:CastFailed
      (Utilities|FlowControl|Delay 0.2)
      (CallFunction|InitPlayerController))))

(event Custom|Init_Toolbar
  (bind _returnvalue (UserInterface|CreateWidget "/Game/WildfyreContent/Widgets/WBP_Wf_Bottom_Bar.WBP_Wf_Bottom_Bar_C" (Game|GetPlayerController 0)))
  (UserInterface|Viewport|AddtoViewport _returnvalue 0)
  (Variables|Default|SetWidgetToolbar _returnvalue))

(event Custom|Init_SelectedActor
  (bind _returnvalue (UserInterface|CreateWidget "/Game/WildfyreContent/Widgets/WBP_Wf_Selected_Actor.WBP_Wf_Selected_Actor_C" (Game|GetPlayerController 0)))
  (UserInterface|Viewport|AddtoViewport _returnvalue 0)
  (Variables|Default|SetWidgetSelectedActor _returnvalue))

(event Custom|Init_WeatherData
  (Utilities|Casting|CastToWfGameStateBase (Game|GetGameState)
    (:then
      (bind _returnvalue (UserInterface|CreateWidget "/Game/WildfyreContent/Widgets/Subelements/W_Data_Clock.W_Data_Clock_C"))
      (UserInterface|Viewport|AddtoViewport _returnvalue 0)
      (Class|UserWidget|SetAnchorsinViewport _returnvalue (Utilities|Struct|MakeAnchors "(X=1.000000,Y=0.000000)" "(X=1.000000,Y=0.000000)"))
      (Layout|BorderSlot|SetPadding _returnvalue (Utilities|Struct|MakeMargin 4.0 4.0 4.0 4.0) :!class /Script/UMG.UserWidget)
      (Class|UserWidget|SetAlignmentinViewport _returnvalue "(X=1.000000,Y=0.000000)")
      (Variables|Default|SetWidgetWeatherData _returnvalue))
    (:CastFailed
      (Utilities|FlowControl|Delay 0.2)
      (CallFunction|InitWeatherData))))

(event Custom|Init_PrimaryMenus
  (bind _aswf_player_state_base (Utilities|Casting|CastToWfPlayerStateBase (Game|GetPlayerState 0))
    (:then
      (Variables|Default|SetPlayerStateRef _aswf_player_state_base)
      (Utilities|FlowControl|Sequence
        (:then_0
          (bind _returnvalue (UserInterface|CreateWidget "/Game/WildfyreContent/Widgets/WBP_Wf_Side_Bar.WBP_Wf_Side_Bar_C" (Game|GetPlayerController 0) 0 (Utilities|Struct|MakeMargin 2.0 2.0 2.0 2.0) (Utilities|Array|MakeArray "/Game/WildfyreContent/Widgets/PrimaryMenus/W_Primary_Menu_Debug.W_Primary_Menu_Debug_C" "/Game/WildfyreContent/Widgets/PrimaryMenus/W_Primary_Menu_Station.W_Primary_Menu_Station_C" "/Game/WildfyreContent/Widgets/PrimaryMenus/W_Primary_Menu_Fleet.W_Primary_Menu_Fleet_C" "/Game/WildfyreContent/Widgets/PrimaryMenus/W_Primary_Menu_Crew.W_Primary_Menu_Crew_C")))
          (bind _output_get (Variables|Default|SetWidgetToolbarSide _returnvalue))
          (UserInterface|Viewport|AddtoViewport _output_get 0))))
    (:CastFailed
      (Utilities|FlowControl|Delay 0.2)
      (CallFunction|InitPrimaryMenus))))

(event EventBeginPlay
  (|CallParentFunction)
  (Utilities|FlowControl|Sequence
    (:then_0
      (bind _returnvalue (UserInterface|CreateWidget "/Game/WildfyreContent/Widgets/WBP_Message_Box.WBP_Message_Box_C" (Game|GetPlayerController 0)))
      (UserInterface|Viewport|AddtoViewport _returnvalue 0)
      (Variables|Default|SetWidgetMessageBox _returnvalue))
    (:then_1
      (CallFunction|InitPlayerController)
      (Utilities|FlowControl|Delay 2.0)
      (CallFunction|SendMessage 0 "Ready!" "The HUD Loaded Successfully" "Error"))))

(fn ConstructionScript)

(fn SendMessage
  (params (MessageIcon :type Texture%202D%20Object%20Reference) (MessageTitle :type String) (MessageBody :type String) (AlertType :type EMessageAlertType%20Enum :default "None"))
  (bind _widgetmessagebox (Variables|Default|GetWidgetMessageBox)
    (:then
      (Default|DisplayMessage _widgetmessagebox (Utilities|Struct|MakeWfMessageData (select (Utilities|IsValid MessageIcon) MessageIcon "/Game/CleanFlatIcons/Textures/png_256/icon_line/icon_line_common/icon_line_common_50.icon_line_common_50") MessageTitle MessageBody AlertType)))
    (:else)))