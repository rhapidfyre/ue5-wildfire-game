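; BP_Wf_Firefighter is the firefighter pawn Blueprint, which sets up a character's name and gendered appearance.
; On BeginPlay it takes the name from the first player controller's display name and binds a gender-set callback before calling the parent BeginPlay.
; The callback compares the gender gameplay tag to Male, then swaps the mesh and animation class between Manny and Quinn.
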(event Custom|Callback_GenderSet
  (params (NewGender :type Gameplay%20Tag%20Structure%20%28by%20ref%29))
  (bind _returnvalue (GameplayTags|MakeLiteralGameplayTag "(TagName=\"Game.Character.Sex.Male\")"))
  (bind _returnvalue_2 (Class|WfCharacterBase|GetCharacterGender))
  (bind _returnvalue_3 (== _returnvalue _returnvalue_2))
  (Components|SkeletalMesh|SetSkeletalMeshAsset (Variables|Character|GetMesh) (select _returnvalue_3 "/Game/Characters/Mannequins/Meshes/SKM_Manny.SKM_Manny" "/Game/Characters/Mannequins/Meshes/SKM_Quinn.SKM_Quinn"))
  (Class|SkeletalMeshComponent|SetAnimClass (Variables|Character|GetMesh) (Class|KismetMathLibrary|SelectClass "/Game/Characters/Mannequins/Animations/ABP_Manny.ABP_Manny_C" "/Game/Characters/Mannequins/Animations/ABP_Quinn.ABP_Quinn_C" _returnvalue_3)))

(event EventBeginPlay
  (Class|WfCharacterBase|SetCharacterName (Utilities|Array|MakeArray (Utilities|GetDisplayName (Game|GetPlayerController 0)) "" ""))
  (EventDispatchers|BindEventtoOnCharacterGenderSet (delegate Custom|Callback_GenderSet))
  (|CallParentFunction))

(fn ConstructionScript)